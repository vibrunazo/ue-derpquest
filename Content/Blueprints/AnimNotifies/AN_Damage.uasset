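; AN_Damage is an anim notify that deals damage around a socket on the animated mesh at the moment it fires.
; It runs a zero-length multi sphere trace for Pawn objects at that socket, using configurable socket name and radius and ignoring the mesh's owner.
; Each hit actor receives the GE_Damage100 effect through the ApplyPickupEffect interface message, with no de-duplication of hits.
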(fn `Received_Notify`
  (params (MeshComp :type "SkeletalMeshComponent Object Reference") (Animation :type "AnimSequenceBase Object Reference") (EventReference :type "AnimNotifyEventReference Structure (by ref)"))
  (returns (ReturnValue :type Boolean))
  (bind _returnvalue (`SceneComponent.GetSocketLocation` MeshComp (`self.SocketName`)))
  (bind (_outhits _returnvalue_2) (`KismetSystemLibrary.SphereTraceMultiForObjects` _returnvalue _returnvalue (`self.SphereRadius`) (`|MakeArray` "ObjectTypeQuery3" :!type "EObjectTypeQuery Enum") false (`|MakeArray` (`ActorComponent.GetOwner` MeshComp))))
  (if _returnvalue_2
    (for _array_element _outhits
      (message `ICanPickup.ApplyPickupEffect` (`.HitActor` (`GameplayStatics.BreakHitResult` _array_element)) "/Game/Blueprints/Abilities/GE_Damage100.GE_Damage100_C"))
    (return true)))