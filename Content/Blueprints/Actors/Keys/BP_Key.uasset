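; BP_Key is a key pickup that, once touched, is flagged to follow whoever collected it.
; Sphere overlap passes KeyTag to any ICanPickup actor, plays a pickup sound, sets that actor as TargetActor and disables the sphere's collision.
; From BeginPlay, it picks a random target offset in a small box, re-rolling at random intervals while ShouldRetriggerOffset is set.
; No movement code consumes these values in these graphs.
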(event `self.Sphere.OnComponentBeginOverlap`
  (params (OverlappedComponent :type "PrimitiveComponent Object Reference") (OtherActor :type "Actor Object Reference") (OtherComp :type "PrimitiveComponent Object Reference") (OtherBodyIndex :type Integer) (bFromSweep :type Boolean) (SweepResult :type "HitResult Structure (by ref)"))
  (bind _asican_pickup (cast `ICanPickup` OtherActor))
  (`ICanPickup.PickupKey` _asican_pickup (`self.Key Tag`))
  (`self.StartFollowPlayer` OtherActor))

(event `ReTriggerRandomOffset`
  (`KismetSystemLibrary.Delay` (`KismetMathLibrary.RandomFloatInRange` 0.8 1.6))
  (`self.SetRandomOffset`))

(event `self.ReceiveBeginPlay`
  (set `self.bShouldMove` true)
  (`self.SetRandomOffset`))

(fn `SetRandomOffset`
  (set `self.TargetOffset` (`KismetMathLibrary.RandomPointInBoundingBox` (0.0 0.0 0.0) (50.0 50.0 50.0)))
  (if (`self.ShouldRetriggerOffset`)
    (`self.ReTriggerRandomOffset`)))

(fn `StartFollowPlayer`
  (params (InputPin :type "Actor Object Reference"))
  (`AudioComponent.Play` (`self.PickupSFX`) 0.0)
  (set `self.TargetActor` InputPin)
  (set `self.bShouldMove` true)
  (`PrimitiveComponent.SetCollisionEnabled` (`self.Sphere`) "NoCollision"))

(fn `UserConstructionScript`)