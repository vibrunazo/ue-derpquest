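; AI controller for Derp characters that gains and loses aggro on the player through perception.
; A sensed DerpCharacter tagged Player is stored as TargetChar on the controlled pawn, and an AI.See event goes to the StateTree.
; Losing sight of that stored target sends AI.Unsee without clearing it.
; FindPlayer and MoveToPlayer are unfinished leftovers that never run.
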(event `self.ReceiveBeginPlay`)

(event `self.PerceptionComponent.OnTargetPerceptionInfoUpdated`
  (params (UpdateInfo :type "ActorPerceptionUpdateInfo Structure (by ref)"))
  (if (`.bSuccessfullySensed` (break `AIStimulus` UpdateInfo_Stimulus))
    (`self.TryAggroAt` UpdateInfo_Target)
    (else
      (`self.TryLoseAggro` UpdateInfo_Target))))

(fn `AggroAt`
  (params (Char :type "DerpCharacter Object Reference"))
  (`self.SetTargetChar` Char)
  (`StateTreeComponent.SendStateTreeEvent` (`self.StateTreeComponent`) (make `StateTreeEvent` (struct :`TagName` "AI.See"))))

(fn `FindPlayer`
  (bind _outactors (`GameplayStatics.GetAllActorsOfClass` "/Script/DerpQuest.DerpCharacter"))
  (for _array_element _outactors
    (`KismetSystemLibrary.IsObjectOfSoftClass` (`Pawn.GetController` _array_element) "/Script/Engine.PlayerController")))

(fn `GetTargetChar`
  (returns (TargetChar :type "DerpCharacter Object Reference"))
  (bind _asderp_character (cast `DerpCharacter` (`self.K2_GetPawn`))
    (:`then`
      (return (`DerpCharacter.TargetChar` _asderp_character)))
    (:`CastFailed`
      (return null))))

(fn `MoveToPlayer`
  (`self.MoveToActor` null -1.0 false true true null))

(fn `SetTargetChar`
  (params (NewTargetChar :type "DerpCharacter Object Reference"))
  (bind _asderp_character (cast `DerpCharacter` (`self.K2_GetPawn`)))
  (set `DerpCharacter.TargetChar` NewTargetChar _asderp_character))

(fn `TryAggroAt`
  (params (Char :type "Actor Object Reference"))
  (bind _asderp_character (cast `DerpCharacter` Char))
  (if (`self.ActorHasTag` _asderp_character "Player")
    (`self.AggroAt` _asderp_character)))

(fn `TryLoseAggro`
  (params (CharLeaving :type "Object Object Reference"))
  (if (== CharLeaving (`self.GetTargetChar`))
    (`StateTreeComponent.SendStateTreeEvent` (`self.StateTreeComponent`) (make `StateTreeEvent` (struct :`TagName` "AI.Unsee")))))

(fn `UserConstructionScript`)